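; BP_Hero is the third-person player character, handling movement, camera look with optional axis inversion, jumping, sprinting and crouching through Enhanced Input.
; Sprint and crouch toggle flags on ABP_Hero and change walk speed directly, without calling the built-in Crouch.
; Debug-style number keys play or reverse a timeline-driven dissolve using a dynamic material on two mesh slots, or spawn an actor at a fixed location.
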(event `self.ReceiveBeginPlay`
  (bind _returnvalue (pcsubsystem `EnhancedInputLocalPlayerSubsystem` (`GameplayStatics.GetPlayerController` 0)))
  (`/Engine/EditorBlueprintResources/StandardMacros.IsValid` _returnvalue
    (:`Is Valid`
      (`EnhancedInputSubsystemInterface.AddMappingContext` _returnvalue "/Game/PlayerSystem/Movement/INC_ThirdPerson.INC_ThirdPerson" 0 (struct)))))

(event `EnhancedInput|/Game/PlayerSystem/Movement/INP_Jump`
  (params (ActionValue :type Boolean) (ElapsedSeconds :type "Float (double-precision)") (TriggeredSeconds :type "Float (double-precision)") (InputAction :type "InputAction Object Reference" :default "/Game/PlayerSystem/Movement/INP_Jump.INP_Jump"))
  (:`Started`
    (`self.Jump`))
  (:`Completed`
    (`self.StopJumping`)))

(event `self.ReceiveTick`
  (params (DeltaSeconds :type "Float (single-precision)")))

(event `EnhancedInput|/Game/PlayerSystem/Movement/INP_MoveAround`
  (params (ActionValue :type "Vector2D Structure") (ElapsedSeconds :type "Float (double-precision)") (TriggeredSeconds :type "Float (double-precision)") (InputAction :type "InputAction Object Reference" :default "/Game/PlayerSystem/Movement/INP_MoveAround.INP_MoveAround"))
  (bind (_returnvalue_roll _returnvalue_pitch _returnvalue_yaw) (`KismetMathLibrary.BreakRotator` (`self.GetControlRotation`)))
  (:`Triggered`
    (`self.AddMovementInput` (`KismetMathLibrary.GetRightVector` (`self.GetControlRotation`)) ActionValue_X)
    (`self.AddMovementInput` (`KismetMathLibrary.GetForwardVector` (`KismetMathLibrary.MakeRotator` _returnvalue_roll 0.0 _returnvalue_yaw)) ActionValue_Y)))

(event `EnhancedInput|/Game/PlayerSystem/Movement/INP_LookAround`
  (params (ActionValue :type "Vector2D Structure") (ElapsedSeconds :type "Float (double-precision)") (TriggeredSeconds :type "Float (double-precision)") (InputAction :type "InputAction Object Reference" :default "/Game/PlayerSystem/Movement/INP_LookAround.INP_LookAround"))
  (:`Triggered`
    (`self.AddControllerYawInput` (* ActionValue_X (`KismetMathLibrary.SelectFloat` -1.0 1.0 (`self.InverCameraX`))))
    (`self.AddControllerPitchInput` (* ActionValue_Y (`KismetMathLibrary.SelectFloat` -1.0 1.0 (`self.InverCameraY`))))))

(event `EnhancedInput|/Game/PlayerSystem/Movement/INP_Run`
  (params (ActionValue :type Boolean) (ElapsedSeconds :type "Float (double-precision)") (TriggeredSeconds :type "Float (double-precision)") (InputAction :type "InputAction Object Reference" :default "/Game/PlayerSystem/Movement/INP_Run.INP_Run"))
  (bind _charactermovement (`self.CharacterMovement`))
  (bind _returnvalue (`SkeletalMeshComponent.GetAnimInstance` (`self.Mesh`)))
  (:`Triggered`
    (bind _asabp_hero (cast `/Game/PlayerSystem/Movement/ABP_Hero` _returnvalue :!label _label))
    (set `/Game/PlayerSystem/Movement/ABP_Hero.Crouch` false _asabp_hero)
    (set `/Game/PlayerSystem/Movement/ABP_Hero.Sprint` true _asabp_hero)
    (set `CharacterMovementComponent.MaxWalkSpeed` 600.0 _charactermovement))
  (:`Ongoing`
    (goto _label))
  (:`Completed`
    (bind _asabp_hero_2 (cast `/Game/PlayerSystem/Movement/ABP_Hero` _returnvalue))
    (set `/Game/PlayerSystem/Movement/ABP_Hero.Sprint` false _asabp_hero_2)
    (set `CharacterMovementComponent.MaxWalkSpeed` 200.0 _charactermovement)))

(event `EnhancedInput|/Game/PlayerSystem/Movement/INP_Crouch`
  (params (ActionValue :type Boolean) (ElapsedSeconds :type "Float (double-precision)") (TriggeredSeconds :type "Float (double-precision)") (InputAction :type "InputAction Object Reference" :default "/Game/PlayerSystem/Movement/INP_Crouch.INP_Crouch"))
  (bind _charactermovement (`self.CharacterMovement`))
  (bind _returnvalue (`SkeletalMeshComponent.GetAnimInstance` (`self.Mesh`)))
  (:`Started`
    (bind _asabp_hero (cast `/Game/PlayerSystem/Movement/ABP_Hero` _returnvalue))
    (if (`/Game/PlayerSystem/Movement/ABP_Hero.Crouch` _asabp_hero)
      (bind _asabp_hero_2 (cast `/Game/PlayerSystem/Movement/ABP_Hero` _returnvalue))
      (set `/Game/PlayerSystem/Movement/ABP_Hero.Crouch` false _asabp_hero_2)
      (set `CharacterMovementComponent.MaxWalkSpeed` 200.0 _charactermovement)
      (else
        (bind _asabp_hero_3 (cast `/Game/PlayerSystem/Movement/ABP_Hero` _returnvalue))
        (set `/Game/PlayerSystem/Movement/ABP_Hero.Crouch` true _asabp_hero_3)
        (set `CharacterMovementComponent.MaxWalkSpeed` 100.0 _charactermovement)))))

(event `Key|One`
  (params (Key :type "Key Structure"))
  (:`Pressed`
    (bind _returnvalue (`PrimitiveComponent.CreateDynamicMaterialInstance` (`self.Mesh`) 0 "/Game/PlayerSystem/Dissolve/DissolveTest_Inst.DissolveTest_Inst" "None"))
    (bind _output_get (set `self.DynamicMat` _returnvalue))
    (bind (_direction _amount) (`Timeline|Dissolve` :!label _label_2)
      (:`Update`
        (`MaterialInstanceDynamic.SetScalarParameterValue` _output_get "Amount" _amount)
        (for _index (range 2)
          (`PrimitiveComponent.SetMaterialByName` (`self.Mesh`) (`|GetArrayItem` (`MeshComponent.GetMaterialSlotNames` (`self.Mesh`)) _index) (`self.DynamicMat`)))))))

(event `Key|Two`
  (params (Key :type "Key Structure"))
  (:`Pressed`
    (goto _label_2 :!via `Reverse`)))

(event `Key|Three`
  (params (Key :type "Key Structure"))
  (:`Pressed`
    (`|SpawnActorFromClass` "/Game/PlayerSystem/BP_TestObject.BP_TestObject_C" (`KismetMathLibrary.MakeTransform` (890.0 1300.0 90.0)) "Undefined" "MultiplyWithRoot" null null)))

(fn `UserConstructionScript`)