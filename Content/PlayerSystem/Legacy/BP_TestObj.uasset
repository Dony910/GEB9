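; BP_TestObj is a legacy test character for morphing: a controllable form the player can leave to return to their original pawn.
; It handles Enhanced Input movement, jumping and invertible camera look.
; A timeline drives a dissolve material across all mesh slots; Moprh reverses it and activates the camera.
; Key 2 dissolves it, teleports the cached player pawn here, messages and repossesses it, then parks this actor at world origin.
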(event `self.ReceiveBeginPlay`
  (bind _returnvalue (pcsubsystem `EnhancedInputLocalPlayerSubsystem` (`GameplayStatics.GetPlayerController` 0)))
  (`self.Dissolve`)
  (`ActorComponent.Deactivate` (`self.Camera`))
  (`/Engine/EditorBlueprintResources/StandardMacros.IsValid` _returnvalue
    (:`Is Valid`
      (`EnhancedInputSubsystemInterface.AddMappingContext` _returnvalue "/Game/PlayerSystem/Movement/INC_ThirdPerson.INC_ThirdPerson" 0 (struct))
      (set `self.Player` (`GameplayStatics.GetPlayerPawn` 0)))))

(event `EnhancedInput|/Game/PlayerSystem/Movement/INP_Jump`
  (params (ActionValue :type Boolean) (ElapsedSeconds :type "Float (double-precision)") (TriggeredSeconds :type "Float (double-precision)") (InputAction :type "InputAction Object Reference" :default "/Game/PlayerSystem/Movement/INP_Jump.INP_Jump"))
  (:`Started`
    (`self.Jump`))
  (:`Completed`
    (`self.StopJumping`)))

(event `EnhancedInput|/Game/PlayerSystem/Movement/INP_MoveAround`
  (params (ActionValue :type "Vector2D Structure") (ElapsedSeconds :type "Float (double-precision)") (TriggeredSeconds :type "Float (double-precision)") (InputAction :type "InputAction Object Reference" :default "/Game/PlayerSystem/Movement/INP_MoveAround.INP_MoveAround"))
  (bind (_returnvalue_roll _returnvalue_pitch _returnvalue_yaw) (`KismetMathLibrary.BreakRotator` (`self.GetControlRotation`)))
  (:`Triggered`
    (`self.AddMovementInput` (`KismetMathLibrary.GetRightVector` (`self.GetControlRotation`)) ActionValue_X)
    (`self.AddMovementInput` (`KismetMathLibrary.GetForwardVector` (`KismetMathLibrary.MakeRotator` _returnvalue_roll 0.0 _returnvalue_yaw)) ActionValue_Y)))

(event `Key|Two`
  (params (Key :type "Key Structure"))
  (bind _player (`self.Player`))
  (bind _returnvalue_location (`KismetMathLibrary.BreakTransform` (`self.GetTransform` self)))
  (:`Pressed`
    (`self.Dissolve`)
    (`self.K2_SetActorLocation` (`self.Player`) _returnvalue_location false true)
    (bind `_as폰` (cast `Pawn` _player))
    (message `/Game/PlayerSystem/Dissolve/BPI_Dissolve.Moprh` _player)
    (`ActorComponent.Deactivate` (`self.Camera`))
    (`KismetSystemLibrary.Delay` 2.0)
    (`Controller.Possess` (`GameplayStatics.GetPlayerController` 0) `_as폰`)
    (`self.K2_SetActorLocation` (0.0 0.0 0.0))
    (`ActorComponent.Deactivate` (`self.Camera`))))

(event `EnhancedInput|/Game/PlayerSystem/Movement/INP_LookAround`
  (params (ActionValue :type "Vector2D Structure") (ElapsedSeconds :type "Float (double-precision)") (TriggeredSeconds :type "Float (double-precision)") (InputAction :type "InputAction Object Reference" :default "/Game/PlayerSystem/Movement/INP_LookAround.INP_LookAround"))
  (:`Triggered`
    (`self.AddControllerYawInput` (* ActionValue_X (`KismetMathLibrary.SelectFloat` -1.0 1.0 (`self.InverCameraX`))))
    (`self.AddControllerPitchInput` (* ActionValue_Y (`KismetMathLibrary.SelectFloat` -1.0 1.0 (`self.InverCameraY`))))))

(event `self.Moprh`
  (`KismetSystemLibrary.Delay` 0.2)
  (`self.UnDissolve`)
  (`ActorComponent.Activate` (`self.Camera`) false))

(event `self.Dissolve`
  (bind _returnvalue (`PrimitiveComponent.CreateDynamicMaterialInstance` (`self.Mesh`) 0 "/Game/PlayerSystem/Dissolve/DissolveTest_Inst.DissolveTest_Inst" "None"))
  (bind _output_get (set `self.DynamicMat` _returnvalue))
  (bind (_direction _amount) (`Timeline|Timeline` :!label _label)
    (:`Update`
      (`MaterialInstanceDynamic.SetScalarParameterValue` _output_get "Amount" _amount)
      (for _index (range (`PrimitiveComponent.GetNumMaterials` (`self.Mesh`)))
        (`PrimitiveComponent.SetMaterialByName` (`self.Mesh`) (`|GetArrayItem` (`MeshComponent.GetMaterialSlotNames` (`self.Mesh`)) _index) (`self.DynamicMat`))))))

(event `self.UnDissolve`
  (goto _label :!via `Reverse`))

(fn `UserConstructionScript`)