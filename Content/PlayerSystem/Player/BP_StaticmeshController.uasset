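; Attached helper actor that lets BP_Hero transform into a copy of a static mesh in the world.
; BeginPlay spawns a movable StaticMeshActor that follows the hero's mesh every tick.
; ChangeStaticMesh copies mesh and scale from the given actor or a camera trace, swapping visibility and gravity, or reverts without a valid target.
; Each tick it syncs transform state to OurPlayerController and restores the hero when TransformStamina hits zero.
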(event `self.ReceiveTick`
  (params (DeltaSeconds :type "Float (single-precision)"))
  (`SceneComponent.K2_SetWorldTransform` (`StaticMeshActor.StaticMeshComponent` (`self.StaticMesh`)) (`SceneComponent.K2_GetComponentToWorld` (`Character.Mesh` (`self.parent`))) false false)
  (`self.SetTransformStamina`))

(event `self.ReceiveBeginPlay`
  (bind _asbp_hero (cast `/Game/PlayerSystem/Player/BP_Hero` (`self.GetAttachParentActor`)))
  (set `self.parent` _asbp_hero)
  (bind _returnvalue (`|SpawnActorFromClass` "/Script/Engine.StaticMeshActor" (`self.GetTransform` self) "Undefined" "MultiplyWithRoot" null null))
  (set `self.StaticMesh` _returnvalue)
  (`AddComponent|NODE_AddChildActorComponent-0` :`self` _returnvalue)
  (`SceneComponent.SetMobility` (`Actor.RootComponent` _returnvalue) "Movable"))

(fn `ChangeStaticMesh`
  (params (InteractedActor :type "Actor Object Reference"))
  (bind _parent (`self.parent`))
  (bind _staticmesh (`self.StaticMesh`))
  (bind _parent_2 (`self.parent`))
  (bind _staticmeshcomponent (`StaticMeshActor.StaticMeshComponent` _staticmesh))
  (bind _staticmeshcomponent_2 (`StaticMeshActor.StaticMeshComponent` (`self.StaticMesh`)))
  (bind _rootcomponent (`Actor.RootComponent` _staticmesh))
  (bind _staticmeshcomponent_3 (`StaticMeshActor.StaticMeshComponent` (`self.StaticMesh`)))
  (bind _mesh (`Character.Mesh` _parent_2))
  (bind _capsulecomponent (`Character.CapsuleComponent` _parent_2))
  (bind `_as스태틱_메시_액터` (cast `StaticMeshActor` InteractedActor)
    (:`then`
      (`KismetSystemLibrary.PrintString` "Hello")
      (bind _staticmeshcomponent_4 (`StaticMeshActor.StaticMeshComponent` `_as스태틱_메시_액터`))
      (`StaticMeshComponent.SetStaticMesh` _staticmeshcomponent_2 (`StaticMeshComponent.StaticMesh` _staticmeshcomponent_4))
      (`SceneComponent.SetWorldScale3D` _staticmeshcomponent_2 (`SceneComponent.K2_GetComponentScale` _staticmeshcomponent_4))
      (`SceneComponent.SetVisibility` _mesh false false :!label _label)
      (`PrimitiveComponent.SetEnableGravity` _capsulecomponent false)
      (`SceneComponent.SetVisibility` _rootcomponent true false)
      (`PrimitiveComponent.SetCollisionResponseToChannel` _staticmeshcomponent "ECC_Camera" "ECR_Overlap")
      (`PrimitiveComponent.SetCollisionResponseToChannel` _staticmeshcomponent "ECC_Pawn" "ECR_Overlap")
      (`PrimitiveComponent.SetCollisionResponseToChannel` _staticmeshcomponent "ECC_Visibility" "ECR_Ignore")
      (`PrimitiveComponent.SetEnableGravity` _staticmeshcomponent true)
      (set `self.isStaticTransform` true))
    (:`CastFailed`
      (bind _interactcomponent (`/Game/PlayerSystem/Player/BP_Hero.LineTraceToComponent` _parent (`/Game/PlayerSystem/Player/BP_Hero.Camera` _parent) 2000 true))
      (`KismetSystemLibrary.PrintString` (`KismetSystemLibrary.GetDisplayName` _interactcomponent))
      (bind `_as스태틱_메시_컴포넌트` (cast `StaticMeshComponent` _interactcomponent)
        (:`then`
          (`StaticMeshComponent.SetStaticMesh` _staticmeshcomponent_3 (`StaticMeshComponent.StaticMesh` `_as스태틱_메시_컴포넌트`))
          (`SceneComponent.SetWorldScale3D` _staticmeshcomponent_3 (`SceneComponent.K2_GetComponentScale` `_as스태틱_메시_컴포넌트`))
          (goto _label))
        (:`CastFailed`
          (`SceneComponent.SetVisibility` _mesh true false)
          (`PrimitiveComponent.SetEnableGravity` _capsulecomponent true)
          (`SceneComponent.SetVisibility` _rootcomponent false false)
          (set `self.isStaticTransform` false))))))

(fn `SetTransformStamina`
  (bind _parent (`self.parent`))
  (bind _asour_player_controller (cast `/Game/PlayerSystem/Player/OurPlayerController` (`GameplayStatics.GetPlayerController` 0)))
  (bind _output_get (set `/Game/PlayerSystem/Player/OurPlayerController.IsstaticmeshTransform` (`self.isStaticTransform`) _asour_player_controller))
  (if (or (not _output_get) (== (`/Game/PlayerSystem/Player/OurPlayerController.transformStamina` _asour_player_controller) 0.0))
    (`SceneComponent.SetVisibility` (`Character.Mesh` _parent) true false)
    (`PrimitiveComponent.SetEnableGravity` (`Character.CapsuleComponent` _parent) true)
    (`SceneComponent.SetVisibility` (`Actor.RootComponent` (`self.StaticMesh`)) false false)
    (set `self.isStaticTransform` false)))

(fn `UserConstructionScript`)