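; Inventory component for the hero that holds item stacks in a fixed-size slot array and handles interaction with world items.
; Each tick it sphere-traces forward from player character 0 to track the looked-at actor, which Interact input sends to a server event that calls its item data component.
; Adding fills matching stacks one unit at a time up to data-table stack sizes, then uses empty slots.
; Removal is an empty stub.
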(event `self.ReceiveBeginPlay`
  (`KismetArrayLibrary.Array_Resize` (`self.content`) (`self.InventorySize`)))

(event `self.ReceiveTick`
  (params (DeltaSeconds :type "Float (single-precision)"))
  (`self.InteractionTrace`))

(event `InputAction|Interact`
  (params (Key :type "Key Structure"))
  (:`Pressed`
    (bind _lookatactor (`self.LookAtActor`)
      (:`then`
        (`self.Server_Interact` _lookatactor))
      (:`else`))))

(event `Server_Interact`
  (params (Target :type "Actor Object Reference"))
  (bind _returnvalue (`Actor.GetComponentByClass` Target "/Game/PlayerSystem/Inventory/BP_ItemDataComponent.BP_ItemDataComponent_C"))
  (`/Engine/EditorBlueprintResources/StandardMacros.IsValid` _returnvalue
    (:`Is Valid`
      (message `/Game/PlayerSystem/Inventory/I_InteractInterface.InteractWith` _returnvalue (cast `/Game/PlayerSystem/BP_Hero` (`self.GetOwner`) :!pure true)))))

(event `Key|One`
  (params (Key :type "Key Structure")))

(fn `AddToInventory`
  (params (ItemID :type Name) (Quantity :type Integer))
  (returns (Success :type Boolean) (QuantityRemaining :type Integer))
  (locals (Local_QuantityRemaining :type Integer) (Local_HasFailed :type Boolean))
  (set `local.Local_QuantityRemaining` Quantity)
  (while (and (> (`local.Local_QuantityRemaining`) 0) (not (`local.Local_HasFailed`)))
    (bind (_index _foundslot) (`self.FindSlot` (`local.ItemID`)))
    (if _foundslot
      (`self.AddToStack` _index 1)
      (`/Engine/EditorBlueprintResources/StandardMacros.DecrementInt` (`local.Local_QuantityRemaining`))
      (elif (`self.AnyEmptySlotsAvailable`)
        (bind _success (`self.CreateNewStack` (`local.ItemID`) 1))
        (if _success
          (`/Engine/EditorBlueprintResources/StandardMacros.DecrementInt` (`local.Local_QuantityRemaining`)))
        (else
          (set `local.Local_HasFailed` true)))))
  (return (not (`local.Local_HasFailed`)) (`local.Local_QuantityRemaining`)))

(fn `AddToStack`
  (params (Index :type Integer) (Quantity :type Integer))
  (bind (_output_itemid _output_quanity) (break `/Game/PlayerSystem/Inventory/FSlotStruct` (`|GetArrayItem` (`self.content`) Index)))
  (`KismetArrayLibrary.Array_Set` (`self.content`) Index (make `/Game/PlayerSystem/Inventory/FSlotStruct` _output_itemid (+ _output_quanity (`local.Quantity`)))))

(fn `AnyEmptySlotsAvailable`
  (returns (HasEmptySlot :type Boolean) (EmptyIndex :type Integer))
  (for (_array_element _array_index) (`self.content`)
    (if (== (`.Quanity_6_E05750CC443792470ABF2BBF7D42C891` (break `/Game/PlayerSystem/Inventory/FSlotStruct` _array_element)) 0)
      (return true _array_index)))
  (return false -1))

(fn `CreateNewStack`
  (params (ItemID :type Name) (Quantity :type Integer))
  (returns (Success :type Boolean))
  (bind (_hasemptyslot _emptyindex) (`self.AnyEmptySlotsAvailable`))
  (if _hasemptyslot
    (`KismetArrayLibrary.Array_Set` (`self.content`) _emptyindex (make `/Game/PlayerSystem/Inventory/FSlotStruct` (`local.ItemID`) (`local.Quantity`)))
    (return true)
    (else
      (return false))))

(fn `DEBUG_PrintContents`
  (for (_array_element _array_index) (`self.content`)
    (bind (_itemid _quanity) (break `/Game/PlayerSystem/Inventory/FSlotStruct` _array_element))
    (`KismetSystemLibrary.PrintString` (`KismetStringLibrary.Concat_StrStr` (`KismetStringLibrary.Conv_IntToString` _array_index) ": " (`KismetStringLibrary.Conv_NameToString` _itemid) " = " (`KismetStringLibrary.Conv_IntToString` _quanity)))))

(fn `FindSlot`
  (params (ItemID :type Name))
  (returns (Index :type Integer) (FoundSlot :type Boolean))
  (bind _itemid (`local.ItemID`))
  (for (_array_element _array_index) (`self.content`)
    (bind (_itemid_2 _quanity) (break `/Game/PlayerSystem/Inventory/FSlotStruct` _array_element))
    (if (== _itemid_2 _itemid)
      (if (< _quanity (`self.GetMaxStackSize` _itemid))
        (return _array_index true))))
  (return -1 false))

(fn `GetMaxStackSize`
  (params (ItemID :type Name))
  (returns (StackSize :type Integer))
  (bind _returnvalue (`|GetDataTableRow` "/Game/PlayerSystem/Inventory/Item_Data.Item_Data" ItemID)
    (:`then`
      (return (`.StackSize_15_512DF6154FF237E688977CBC629CB397` (break `/Game/PlayerSystem/Inventory/FItemStruct` _returnvalue))))
    (:`RowNotFound`
      (return -1))))

(fn `InteractionTrace`
  (bind _returnvalue (`GameplayStatics.GetPlayerCharacter` 0))
  (bind _returnvalue_2 (`Actor.K2_GetActorLocation` _returnvalue))
  (bind (_outhit _returnvalue_3) (`KismetSystemLibrary.SphereTraceSingle` _returnvalue_2 (+ _returnvalue_2 (* (`Actor.GetActorForwardVector` _returnvalue) (`self.InteractionRange`))) 15.0 "TraceTypeQuery3" false (`|MakeArray` (`self.GetOwner`))))
  (if _returnvalue_3
    (bind (_bblockinghit _binitialoverlap _time _distance _location _impactpoint _normal _impactnormal _physmat _hitactor) (`GameplayStatics.BreakHitResult` _outhit))
    (if (!= _hitactor (`self.LookAtActor`))
      (bind _output_get (set `self.LookAtActor` _hitactor))
      (bind _message (message `/Game/PlayerSystem/Inventory/I_InteractInterface.LookAt` _output_get))
      (`KismetSystemLibrary.PrintString` (`KismetTextLibrary.Conv_TextToString` _message)))
    (else
      (set `self.LookAtActor` null))))

(fn `RemoveFromInventory`)