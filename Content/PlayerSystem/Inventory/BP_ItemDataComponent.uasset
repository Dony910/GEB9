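; BP_ItemDataComponent is an actor component that carries an item ID and quantity for its owning actor, as part of the inventory system.
; On BeginPlay it turns on replication for the owner.
; Its Interactwith event is empty and LookAt returns an empty string.
; Logic to add the item to BPInventorySystem and destroy the owner on success exists but is disconnected, so pickup never runs here.
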(event `self.ReceiveBeginPlay`
  (`Actor.SetReplicates` (`self.GetOwner`) true))

(event `/Game/PlayerSystem/Inventory/I_InteractInterface.InteractWith`
  (params (PlayerCharacter :type "/Game/PlayerSystem/BP_Hero Object Reference")))

(fn `LookAt`
  (returns (Message :type Text))
  (return ""))