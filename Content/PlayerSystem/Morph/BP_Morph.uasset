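; BP_Morph drives a particle-based morph effect from Character1 to Character2.
; On BeginPlay it attaches P_Morph to Character1, binds both skeletal meshes to the Niagara system and animates MPC_Morph's "Amount" down.
; A Niagara export callback compares the first particle's Position against its Velocity field, apparently used as a target point.
; Once they are close, a one-time timeline raises "Amount1".
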(event `self.ReceiveBeginPlay`
  (bind _skeletalmeshcomponent (`SkeletalMeshActor.SkeletalMeshComponent` (`self.Character1`)))
  (bind _returnvalue (`NiagaraFunctionLibrary.SpawnSystemAttached` "/Game/PlayerSystem/Morph/P_Morph.P_Morph" _skeletalmeshcomponent "None" (0.0 0.0 0.0) (struct) "KeepRelativeOffset"))
  (`NiagaraComponent.SetVariableObject` _returnvalue "Callback" self)
  (`NiagaraFunctionLibrary.OverrideSystemUserVariableSkeletalMeshComponent` _returnvalue "Skeletal Mesh" _skeletalmeshcomponent)
  (`NiagaraFunctionLibrary.OverrideSystemUserVariableSkeletalMeshComponent` _returnvalue "Skeletal Mesh001" (`SkeletalMeshActor.SkeletalMeshComponent` (`self.Character2`)))
  (bind (_direction _newtrack_0) (`Timeline|Timeline` :!via `PlayFromStart`)
    (:`Update`
      (`KismetMaterialLibrary.SetScalarParameterValue` "/Game/PlayerSystem/Morph/MPC_Morph.MPC_Morph" "Amount" (`KismetMathLibrary.Lerp` 1.0 0.0 _newtrack_0)))))

(event `self.ReceiveParticleData`
  (params (Data :type "Array of BasicParticleData Structure (by ref)") (NiagaraSystem :type "NiagaraSystem Object Reference") (SimulationPositionOffset :type "Vector Structure (by ref)"))
  (bind (_position _size _velocity) (break `BasicParticleData` (`|GetArrayItem` Data)))
  (if (<= (`KismetMathLibrary.VSize` (- _velocity _position)) 80.0)
    (`/Engine/EditorBlueprintResources/StandardMacros.DoOnce` false
      (:`Completed`
        (bind (_direction _newtrack_0) (`Timeline|Timeline_0` :!via `PlayFromStart`)
          (:`Update`
            (`KismetMaterialLibrary.SetScalarParameterValue` "/Game/PlayerSystem/Morph/MPC_Morph.MPC_Morph" "Amount1" (`KismetMathLibrary.Lerp` 0.0 1.0 _newtrack_0))))))))

(fn `UserConstructionScript`)