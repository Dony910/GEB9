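; BP_enemy is an enemy that uses AI Perception to track the player by sight, sound and CCTV alerts.
; Each tick it accumulates exposed and unexposed time for a visible BP_Hero, and heard and unheard time for any sound.
; Stimuli tagged CCTV set a detection flag, which a retriggerable delay clears after a few seconds.
; It prints these timers, the CCTV flag and the Fsm state for debugging.
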(event `self.ReceiveTick`
  (params (DeltaSeconds :type "Float (single-precision)"))
  (`self.visionProcess` DeltaSeconds)
  (`self.HearingProcess` DeltaSeconds)
  (`|ExecutionSequence`
    (:`then_0`
      (`self.CCTVTimercontrol`))
    (:`then_1`
      (`self.DebugText`))))

(event `self.AIPerception.OnTargetPerceptionUpdated`
  (params (Actor :type "Actor Object Reference") (Stimulus :type "AIStimulus Structure"))
  (`self.CCTVProcess` Stimulus))

(fn `CCTVProcess`
  (params (AIStimulus :type "AIStimulus Structure (by ref)"))
  (if (== (`.Tag` (break `AIStimulus` AIStimulus)) "CCTV")
    (set `self.cctvdetected` true)
    (set `self.cctvTimer` true)))

(fn `DebugText`
  (bind _playerexposedtime (`self.playerExposedTime`))
  (bind _soundheardtime (`self.soundHeardTime`))
  (if (<= _playerexposedtime 0.1)
    (`KismetSystemLibrary.PrintString` (`KismetStringLibrary.Concat_StrStr` "PlayerUnExposedTime : " (`KismetTextLibrary.Conv_TextToString` (`KismetTextLibrary.Conv_DoubleToText` (`self.playerUnExposedTime`) "HalfToEven" false true 1 3)) "s") true false (struct :`G` 0.66 :`B` 1.0 :`A` 1.0) 2.0 "PlayerExposedTime")
    (else
      (`KismetSystemLibrary.PrintString` (`KismetStringLibrary.Concat_StrStr` "PlayerExposedTime : " (`KismetTextLibrary.Conv_TextToString` (`KismetTextLibrary.Conv_DoubleToText` _playerexposedtime "HalfToEven" false true 1 3)) "s") true false (struct :`R` 1.0 :`A` 1.0) 2.0 "PlayerExposedTime")))
  (if (<= _soundheardtime 0.1)
    (`KismetSystemLibrary.PrintString` (`KismetStringLibrary.Concat_StrStr` "SoundUnHeardTime : " (`KismetTextLibrary.Conv_TextToString` (`KismetTextLibrary.Conv_DoubleToText` (`self.soundUnHeardTime`) "HalfToEven" false true 1 3)) "s") true false (struct :`G` 0.66 :`B` 1.0 :`A` 1.0) 2.0 "SoundHeardTime")
    (else
      (`KismetSystemLibrary.PrintString` (`KismetStringLibrary.Concat_StrStr` "SoundHeardTime : " (`KismetTextLibrary.Conv_TextToString` (`KismetTextLibrary.Conv_DoubleToText` _soundheardtime "HalfToEven" false true 1 3)) "s") true false (struct :`R` 1.0 :`A` 1.0) 2.0 "SoundHeardTime")))
  (`KismetSystemLibrary.PrintString` (`KismetStringLibrary.Concat_StrStr` "State : " (`|GetEnumeratorNameAsString` (`EnemyFSM.mstate` (`self.fsm`)))) true true (struct :`G` 0.66 :`B` 1.0 :`A` 1.0) 2.0 "state")
  (`KismetSystemLibrary.PrintString` (`KismetStringLibrary.Concat_StrStr` "cctv detected :" (`KismetStringLibrary.Conv_BoolToString` (`self.cctvdetected`))) true true (struct :`G` 0.66 :`B` 1.0 :`A` 1.0) 2.0 "cctvdetected"))

(fn `HearingProcess`
  (params (InDouble :type "Float (double-precision)"))
  (set `self.IsHeard` false)
  (for _ (`AIPerceptionComponent.GetCurrentlyPerceivedActors` (`self.AIPerception`) "/Script/AIModule.AISense_Hearing")
    (set `self.IsHeard` true))
  (if (`self.IsHeard`)
    (set `self.soundUnHeardTime` 0.0)
    (set `self.soundHeardTime` (+ InDouble (`self.soundHeardTime`)))
    (else
      (set `self.soundHeardTime` 0.0)
      (set `self.soundUnHeardTime` (+ (`self.soundUnHeardTime`) InDouble)))))

(fn `UserConstructionScript`)

(fn `VisionProcess`
  (params (B :type "Float (double-precision)"))
  (set `self.IsPlayerVisible` false)
  (for _array_element (`AIPerceptionComponent.GetCurrentlyPerceivedActors` (`self.AIPerception`) "/Script/AIModule.AISense_Sight")
    (if (== (`GameplayStatics.GetObjectClass` _array_element) "/Game/PlayerSystem/Player/BP_Hero.BP_Hero_C")
      (set `self.IsPlayerVisible` true)))
  (if (`self.IsPlayerVisible`)
    (set `self.playerUnExposedTime` 0.0)
    (set `self.playerExposedTime` (+ (`self.playerExposedTime`) B))
    (else
      (set `self.playerExposedTime` 0.0)
      (set `self.playerUnExposedTime` (+ (`self.playerUnExposedTime`) B)))))