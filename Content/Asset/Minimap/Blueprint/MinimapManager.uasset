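; Minimap manager that gives tagged walls, enemies, heroes and CCTVs overhead marker meshes at BeginPlay.
; Each pass finds actors by class and tag, then adds a static mesh component to each at a fixed height above its colliding-bounds origin.
; Walls get planes scaled from their box extents, enemies planes, heroes cones and CCTVs spheres.
; Markers auto-attach to their actors, so no Tick update is used.
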(event `self.ReceiveBeginPlay`
  (`|ExecutionSequence`
    (:`then_0`
      (`self.wall`))
    (:`then_1`
      (`self.enemy`))
    (:`then_2`
      (bind _outactors (`GameplayStatics.GetAllActorsOfClassWithTag` "/Game/PlayerSystem/Player/BP_Hero.BP_Hero_C" "player"))
      (for _array_element _outactors
        (bind _returnvalue (`AddComponent|NODE_AddStaticMeshComponent-2` :`self` _array_element))
        (`StaticMeshComponent.SetStaticMesh` _returnvalue "/Engine/BasicShapes/Cone.Cone")
        (`SceneComponent.K2_SetWorldTransform` _returnvalue (`KismetMathLibrary.MakeTransform` (`KismetMathLibrary.MakeVector` (.x (`self.GetActorBounds` _array_element true false)) (.y (`self.GetActorBounds` _array_element true false)) (+ (.z (`self.GetActorBounds` _array_element true false)) 800.0))) false false)))
    (:`then_3`
      (bind _outactors_2 (`GameplayStatics.GetAllActorsOfClassWithTag` "/Game/Asset/TransOBJ/CCTV/BluePrint/CCTV.CCTV_C" "CCTV"))
      (for _array_element_2 _outactors_2
        (bind _returnvalue_2 (`AddComponent|NODE_AddStaticMeshComponent-3` :`self` _array_element_2))
        (`StaticMeshComponent.SetStaticMesh` _returnvalue_2 "/Engine/EditorMeshes/ArcadeEditorSphere.ArcadeEditorSphere")
        (`SceneComponent.K2_SetWorldTransform` _returnvalue_2 (`KismetMathLibrary.MakeTransform` (`KismetMathLibrary.MakeVector` (.x (`self.GetActorBounds` _array_element_2 true false)) (.y (`self.GetActorBounds` _array_element_2 true false)) (+ (.z (`self.GetActorBounds` _array_element_2 true false)) 800.0))) false false)))))

(fn `enemy`
  (bind _outactors (`GameplayStatics.GetAllActorsOfClassWithTag` "/Script/Engine.Character" "enemy"))
  (for _array_element _outactors
    (bind _returnvalue (`AddComponent|NODE_AddStaticMeshComponent-1` :`self` _array_element))
    (`StaticMeshComponent.SetStaticMesh` _returnvalue "/Engine/BasicShapes/Plane.Plane")
    (`SceneComponent.K2_SetWorldTransform` _returnvalue (`KismetMathLibrary.MakeTransform` (`KismetMathLibrary.MakeVector` (.x (`self.GetActorBounds` _array_element true false)) (.y (`self.GetActorBounds` _array_element true false)) (+ (.z (`self.GetActorBounds` _array_element true false)) 800.0))) false false)))

(fn `UserConstructionScript`)

(fn `wall`
  (bind _outactors (`GameplayStatics.GetAllActorsOfClassWithTag` "/Script/Engine.StaticMeshActor" "wall"))
  (for _array_element _outactors
    (bind _returnvalue (`AddComponent|NODE_AddStaticMeshComponent-0` :`self` _array_element))
    (`StaticMeshComponent.SetStaticMesh` _returnvalue "/Engine/BasicShapes/Plane.Plane")
    (bind (_origin _boxextent) (`self.GetActorBounds` _array_element true false))
    (`SceneComponent.K2_SetWorldTransform` _returnvalue (`KismetMathLibrary.MakeTransform` (`KismetMathLibrary.MakeVector` (.x _origin) (.y _origin) (+ (.z _origin) 800.0)) (struct) (/ _boxextent 50.0)) false false)))