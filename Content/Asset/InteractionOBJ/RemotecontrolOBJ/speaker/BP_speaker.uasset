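; BP_speaker is a speaker object that makes a noise AI can hear when switched on.
; BeginPlay creates a 2D, non-spatialized audio component from the Collapse01 sound and stores it.
; Toggle uses a FlipFlop to alternate between Active and DisActive.
; Active reports a single noise event tagged "speaker" at the actor's location and plays the sound from the start, while DisActive stops it.
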(event `self.ReceiveBeginPlay`
  (bind _returnvalue (`GameplayStatics.CreateSound2D` "/Game/StarterContent/Audio/Collapse01.Collapse01" 1.0 1.0 0.0 null))
  (set `self.sound` _returnvalue))

(event `self.ReceiveTick`
  (params (DeltaSeconds :type "Float (single-precision)")))

(event `self.Toggle`
  (`/Engine/EditorBlueprintResources/StandardMacros.FlipFlop`
    (:`A`
      (`self.Active`))
    (:`B`
      (`self.DisActive`))))

(event `self.DisActive`
  (`AudioComponent.Stop` (`self.sound`)))

(event `self.Active`
  (`AISense_Hearing.ReportNoiseEvent` (`self.K2_GetActorLocation` self) 1.0 self 0.0 "speaker")
  (`AudioComponent.Play` (`self.sound`) 0.0))

(fn `UserConstructionScript`)