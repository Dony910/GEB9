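; BP_KeyDoor is a two-panel sliding door that responds to Interact only when the BP_Hero found at BeginPlay has the blue key.
; A timeline slides the panels apart along local Y by an offset derived from the left panel's scale, then reverses to close, with sounds for both.
; Opening schedules an automatic close after a delay, which leaves InOpen set, whereas interacting while InOpen closes and clears it.
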(event `self.ReceiveBeginPlay`
  (bind _relativescale3d_x (`KismetMathLibrary.BreakVector` (`SceneComponent.RelativeScale3D` (`self.SM_Doors_Gate_Left`))))
  (set `self.rDoorsInitpos` (`SceneComponent.RelativeLocation` (`self.SM_Doors_Right`)))
  (set `self.lDoorsInitpos` (`SceneComponent.RelativeLocation` (`self.SM_Doors_Gate_Left`)))
  (set `self.moveamount` (* _relativescale3d_x 100.0))
  (bind _returnvalue (`GameplayStatics.GetActorOfClass` "/Game/PlayerSystem/Player/BP_Hero.BP_Hero_C"))
  (set `self.player` _returnvalue))

(event `/Game/Asset/InteractionOBJ/InteractInterface.Interact`
  (if (`/Game/PlayerSystem/Player/BP_Hero.IsBluekey` (`self.player`))
    (if (`self.InOpen`)
      (`/Game/Asset/InteractionOBJ/InteractInterface.disactive`)
      (set `self.InOpen` false)
      (set `self.IsOpen` false)
      (else
        (`/Game/Asset/InteractionOBJ/InteractInterface.active`)
        (set `self.InOpen` true)
        (`KismetSystemLibrary.Delay` 3.0)
        (`/Game/Asset/InteractionOBJ/InteractInterface.disactive`)))))

(event `/Game/Asset/InteractionOBJ/InteractInterface.active`
  (bind _moveamount (`self.moveamount`))
  (`GameplayStatics.PlaySoundAtLocation` "/Game/SFX/Environment/Door_Open.Door_Open" (`self.K2_GetActorLocation`) (struct) 1.0 1.0 0.0 "/Game/Asset/sound/linearattenuation.linearattenuation" null null null)
  (bind (_direction _amount) (`Timeline|타임라인` :!label _label)
    (:`Update`
      (`SceneComponent.K2_SetRelativeLocation` (`self.SM_Doors_Right`) (+ (`self.rDoorsInitpos`) (`KismetMathLibrary.MakeVector` 0.0 (* _amount _moveamount 0.01))) false false)
      (`SceneComponent.K2_SetRelativeLocation` (`self.SM_Doors_Gate_Left`) (+ (`self.lDoorsInitpos`) (`KismetMathLibrary.MakeVector` 0.0 (* _amount _moveamount -0.01))) false false))
    (:`Finished`
      (if (`self.InOpen`)
        (set `self.IsOpen` true)))))

(event `/Game/Asset/InteractionOBJ/InteractInterface.disactive`
  (`GameplayStatics.PlaySoundAtLocation` "/Game/SFX/Environment/Door_Close.Door_Close" (`self.K2_GetActorLocation`) (struct) 1.0 1.0 0.0 "/Game/Asset/sound/linearattenuation.linearattenuation" null null null)
  (goto _label :!via `Reverse`))

(fn `UserConstructionScript`)