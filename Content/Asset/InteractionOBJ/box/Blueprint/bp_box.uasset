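; Interactable box Blueprint that toggles open and closed each time Interact is called.
; Active plays the Boxopen timeline and Disactive reverses it, with each update writing a scaled angle into YawAngle on the abp_box Animation Blueprint.
; InOpen tracks the requested state, while IsOpen becomes true only when opening finishes and clears as soon as closing starts.
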(event `/Game/Asset/InteractionOBJ/InteractInterface.Interact`
  (if (`self.InOpen`)
    (`/Game/Asset/InteractionOBJ/InteractInterface.disactive`)
    (set `self.InOpen` false)
    (set `self.IsOpen` false)
    (else
      (`/Game/Asset/InteractionOBJ/InteractInterface.active`)
      (set `self.InOpen` true))))

(event `/Game/Asset/InteractionOBJ/InteractInterface.active`
  (bind (_direction _angle) (`Timeline|boxopen` :!label _label)
    (:`Update`
      (set `/Game/Asset/InteractionOBJ/Box/Blueprint/abp_box.yawAngle` (* _angle 0.6) (cast `/Game/Asset/InteractionOBJ/Box/Blueprint/abp_box` (`SkeletalMeshComponent.GetAnimInstance` (`self.SkeletalMesh`)) :!pure true)))
    (:`Finished`
      (if (`self.InOpen`)
        (set `self.IsOpen` true)))))

(event `/Game/Asset/InteractionOBJ/InteractInterface.disactive`
  (goto _label :!via `Reverse`))

(fn `UserConstructionScript`)