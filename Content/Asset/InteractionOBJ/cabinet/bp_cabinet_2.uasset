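; Interactable cabinet Blueprint whose lid or door, CabinetRid, swings open and closed on interaction.
; Interact toggles the InOpen flag and calls Active or Disactive.
; Active plays the Boxopen timeline, whose Angle track is negated into the relative yaw of CabinetRid, and Disactive reverses that timeline.
; IsOpen is only cleared on closing, and the timeline's Finished branch does nothing.
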(event `/Game/Asset/InteractionOBJ/InteractInterface.Interact`
  (if (`self.InOpen`)
    (`/Game/Asset/InteractionOBJ/InteractInterface.disactive`)
    (set `self.InOpen` false)
    (set `self.IsOpen` false)
    (else
      (`/Game/Asset/InteractionOBJ/InteractInterface.active`)
      (set `self.InOpen` true))))

(event `/Game/Asset/InteractionOBJ/InteractInterface.active`
  (bind (_direction _angle) (`Timeline|boxopen` :!label _label)
    (:`Update`
      (`SceneComponent.K2_SetRelativeRotation` (`self.Cabinet_rid`) (`KismetMathLibrary.MakeRotator` 0.0 0.0 (* _angle -1.0)) false false))
    (:`Finished`
      (if (`self.InOpen`)
        _))))

(event `/Game/Asset/InteractionOBJ/InteractInterface.disactive`
  (goto _label :!via `Reverse`))

(fn `UserConstructionScript`)