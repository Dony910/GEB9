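; BP_EnemyUI is an enemy state indicator actor that shows its parent BP_enemy's AI state as a color.
; BeginPlay creates a dynamic material on the EnmeyUI component, sets its radius parameter and caches the parent enemy.
; Tick maps the enemy's FSM state (Patrol, Alert, Check, Chase, Return, Neutralize) to a color and writes it to the material's color parameter every frame.
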(event `self.ReceiveBeginPlay`
  (bind _returnvalue (`PrimitiveComponent.CreateDynamicMaterialInstance` (`self.EnmeyUI`) 0 "/Game/Asset/HostileOBJ/enemy/Mat_EnemyUIinstance.Mat_EnemyUIinstance" "None"))
  (bind _output_get (set `self.DynamicUI` _returnvalue))
  (`MaterialInstanceDynamic.SetScalarParameterValue` _output_get "radius" 0.5)
  (bind _asbp_enemy (cast `/Game/Asset/HostileOBJ/enemy/BP_enemy` (`self.GetParentActor`)))
  (set `self.Enemy` _asbp_enemy))

(event `self.ReceiveTick`
  (params (DeltaSeconds :type "Float (single-precision)"))
  (`|ExecutionSequence`
    (:`then_0`
      (switch `EEnemyState` (`EnemyFSM.mstate` (`Enemy.fsm` (`self.Enemy`)))
        (:`Patrol`
          (set `self.color` (struct :`R` 0.302199 :`G` 0.995 :`B` 0.902627 :`A` 1.0)))
        (:`Alert`
          (set `self.color` (struct :`R` 1.0 :`G` 0.788692 :`A` 1.0)))
        (:`Check`
          (set `self.color` (struct :`R` 1.0 :`G` 0.305141 :`A` 1.0)))
        (:`Chase`
          (set `self.color` (struct :`R` 0.818 :`G` 0.01502 :`A` 1.0)))
        (:`Return`
          (set `self.color` (struct :`R` 0.551 :`G` 0.608457 :`B` 1.0 :`A` 1.0)))
        (:`Neutralize`
          (set `self.color` (struct)))))
    (:`then_1`
      (`MaterialInstanceDynamic.SetVectorParameterValue` (`self.DynamicUI`) "color" (`self.color`)))))

(fn `UserConstructionScript`)