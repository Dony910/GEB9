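; BP_CCTVUI is the visual indicator for a CCTV's vision cone, expecting that CCTV as its parent actor.
; On BeginPlay it creates a dynamic material instance and sets its radius and angle from the camera's cone length and visible FOV.
; Each Tick it sets the indicator's world yaw from the mesh's cctv_socket, with a fixed offset, so the cone follows the camera's heading.
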(event `self.ReceiveBeginPlay`
  (bind _cctv (`self.CCTV`))
  (bind _ascctv (cast `/Game/Asset/HostileOBJ/CCTV/BluePrint/CCTV` (`self.GetParentActor`)))
  (set `self.CCTV` _ascctv)
  (bind _returnvalue (`PrimitiveComponent.CreateDynamicMaterialInstance` (`self.CCTVvisionUI`) 0 "/Game/Asset/HostileOBJ/CCTV/Material/CCTVUI_Inst.CCTVUI_Inst" "None"))
  (bind _output_get (set `self.DynamicUI` _returnvalue))
  (`MaterialInstanceDynamic.SetScalarParameterValue` _output_get "radius" (/ (* (`/Game/Asset/HostileOBJ/CCTV/BluePrint/CCTV.VisionconeLength` _cctv) 0.1) 200.0))
  (`MaterialInstanceDynamic.SetScalarParameterValue` _output_get "angle" (`CCTVbase.visibleFOV` _cctv)))

(event `self.ReceiveTick`
  (params (DeltaSeconds :type "Float (single-precision)"))
  (`SceneComponent.K2_SetWorldRotation` (`self.CCTVvisionUI`) (`KismetMathLibrary.MakeRotator` 0.0 0.0 (- (.yaw (.rotation (`SceneComponent.GetSocketTransform` (`Character.Mesh` (`self.CCTV`)) "cctv_socket" "RTS_World"))) 90.0)) false false))

(fn `UserConstructionScript`)