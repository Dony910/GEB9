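; CCTV camera actor that sweeps back and forth, with a vision cone that follows it.
; Each tick CameraMove passes yaw, pitch and current angle to ABP_CCTV, ping-ponging the angle between plus and minus RotationAngle at a rate derived from RotationPeriod.
; Visionconetransform then rebuilds the cone from the mesh's socket and bone rotation, sizing it by VisionconeLength and the tangent of RotationAngle.
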(event `self.ReceiveBeginPlay`)

(event `self.ReceiveTick`
  (params (DeltaSeconds :type "Float (single-precision)"))
  (`self.CameraMove` DeltaSeconds)
  (`self.Visionconetransform`))

(fn `CameraMove`
  (params (A :type "Float (double-precision)"))
  (bind _currentangle (`self.CurrentAngle`))
  (bind _returnvalue (* A (/ 1.0 (`self.RotationPeriod`)) (`self.RotationAngle`) 4.0))
  ;[1 1 1] Check having Valid ABP
  (bind _asabp_cctv (cast `/Game/Asset/CCTV/BluePrint/ABP_CCTV` (`SkeletalMeshComponent.GetAnimInstance` (`self.Mesh`))))
  (if true
    ;[1 1 1] default pose set
    (set `/Game/Asset/CCTV/BluePrint/ABP_CCTV.yawAngle` (`self.yawAngle`) _asabp_cctv)
    (set `/Game/Asset/CCTV/BluePrint/ABP_CCTV.pitchAngle` (`self.pitchAngle`) _asabp_cctv)
    ;[1 1 1] modify Angle
    (set `/Game/Asset/CCTV/BluePrint/ABP_CCTV.rotationAngle` (`self.CurrentAngle`) _asabp_cctv)
    (if (`self.Direction`)
      (bind _output_get (set `self.currentAngle` (- _currentangle _returnvalue)))
      (if (>= (* (`self.RotationAngle`) -1.0) _output_get)
        (set `self.direction` false))
      (else
        (bind _output_get_2 (set `self.currentAngle` (+ _currentangle _returnvalue)))
        (if (>= _output_get_2 (`self.RotationAngle`))
          (set `self.direction` true))))))

(fn `UserConstructionScript`)

(fn `Visionconetransform`
  (bind _visioncone (`self.VisionCone`))
  (bind _mesh (`self.Mesh`))
  (bind _returnvalue (`SceneComponent.GetSocketLocation` _mesh "cctv_socket"))
  (bind _returnvalue_2 (/ (`self.VisionconeLength`) 100.0))
  (bind _returnvalue_3 (* (`KismetMathLibrary.DegTan` (`self.RotationAngle`)) _returnvalue_2))
  (`SceneComponent.K2_SetWorldTransform` _visioncone (`KismetMathLibrary.MakeTransform` _returnvalue (struct :`Roll` 90.0) (`KismetMathLibrary.MakeVector` _returnvalue_3 _returnvalue_3 _returnvalue_2)) false false)
  (`SceneComponent.K2_AddWorldRotation` _visioncone (`SceneComponent.GetSocketRotation` _mesh "Bone_003") false false)
  (`SceneComponent.K2_AddLocalOffset` _visioncone (`KismetMathLibrary.MakeVector` 0.0 0.0 (* (`KismetMathLibrary.Vector_Distance` _returnvalue (`SceneComponent.GetSocketLocation` (`self.VisionCone`) "Origin")) -1.0)) false false))