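; BP_CCTV is a security camera actor whose skeletal mesh sweeps back and forth.
; Each Tick, it advances CurrentAngle at a rate set by RotationAngle and RotationPeriod, flipping Direction at either limit to form a ping-pong sweep.
; It pushes that angle and a YawAngle into the mesh's ABP_CCTV Animation Blueprint as RotationAngle and YawAngle, leaving the pose to the anim instance.
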(event `self.ReceiveTick`
  (params (DeltaSeconds :type "Float (single-precision)"))
  (bind _currentangle (`self.currentAngle`))
  (bind _returnvalue (* DeltaSeconds (/ 1.0 (`self.rotationPeriod`)) (`self.rotationAngle`) 4.0))
  (bind _asabp_cctv (cast `/Game/Asset/CCTV/ABP_CCTV` (`SkeletalMeshComponent.GetAnimInstance` (`self.SkeletalMesh`))))
  (if true
    (set `/Game/Asset/CCTV/ABP_CCTV.yawAngle` (`self.yawAngle`) _asabp_cctv)
    (set `/Game/Asset/CCTV/ABP_CCTV.rotationAngle` (`self.currentAngle`) _asabp_cctv)
    (if (`self.direction`)
      (bind _output_get (set `self.currentAngle` (- _currentangle _returnvalue)))
      (if (>= (* (`self.rotationAngle`) -1.0) _output_get)
        (set `self.direction` false))
      (else
        (bind _output_get_2 (set `self.currentAngle` (+ _currentangle _returnvalue)))
        (if (>= _output_get_2 (`self.rotationAngle`))
          (set `self.direction` true))))))

(fn `UserConstructionScript`)